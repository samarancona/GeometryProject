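; BP_WallGeometrical is a Geometry Script wall that first-person projectiles deform on impact, apparently to punch holes.
; Mesh rebuild generates a box from the dimension variables and applies PN tessellation, storing the result as TargetMesh.
; On a projectile hit, it copies and simplifies RefMesh in a pooled compute mesh.
; That tool mesh is applied with a configurable boolean at the local hit location, scaled by projectile speed over HoleScale.
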(event `self.OnRebuildGeneratedMesh`
  (params (TargetMesh :type "DynamicMesh Object Reference"))
  (bind _returnvalue (`GeometryScriptLibrary_MeshPrimitiveFunctions.AppendBox` TargetMesh (struct) (struct) (`self.Dimension X`) 50.0 (`self.Dimension Z`) 0 0 0 "Base" null))
  (bind _returnvalue_2 (`GeometryScriptLibrary_MeshSubdivideFunctions.ApplyPNTessellation` _returnvalue (struct) (`self.Tessellation Level`) null))
  (set `self.Target Mesh` _returnvalue_2))

(event `self.DynamicMeshComponent.OnComponentHit`
  (params (HitComponent :type "PrimitiveComponent Object Reference") (OtherActor :type "Actor Object Reference") (OtherComp :type "PrimitiveComponent Object Reference") (NormalImpulse :type "Vector Structure") (Hit :type "HitResult Structure (by ref)"))
  (bind _operation (`self.Operation`))
  (bind _ref_mesh (`self.Ref Mesh`))
  (bind _target_mesh (`self.Target Mesh`))
  (bind _returnvalue (`KismetMathLibrary.InverseTransformLocation` (`SceneComponent.K2_GetComponentToWorld` (`self.DynamicMeshComponent`)) (`.Location` (`GameplayStatics.BreakHitResult` Hit))))
  (bind _asbp_first_person_projectile (cast `/Game/FirstPerson/Blueprints/BP_FirstPersonProjectile` OtherActor))
  (`/Engine/EditorBlueprintResources/StandardMacros.IsValid` (`self.Dynamic Mesh Projectile`)
    (:`Is Valid`
      (bind _returnvalue_2 (`self.AllocateComputeMesh`))
      (bind _returnvalue_3 (`GeometryScriptLibrary_StaticMeshFunctions.CopyMeshFromStaticMesh` _ref_mesh _returnvalue_2 (make `GeometryScriptCopyMeshFromAssetOptions` true) (struct) null)
        (:`Success`
          (bind _returnvalue_4 (`GeometryScriptLibrary_MeshSimplifyFunctions.ApplySimplifyToTriangleCount` _returnvalue_3 0 (struct) null))
          (bind _returnvalue_5 (`GeometryScriptLibrary_MeshSimplifyFunctions.ApplySimplifyToVertexCount` _returnvalue_4 0 (struct) null))
          (bind _returnvalue_6 (/ (`KismetMathLibrary.VSize` (`self.GetVelocity` _asbp_first_person_projectile)) (`self.HoleScale`)))
          (`GeometryScriptLibrary_MeshBooleanFunctions.ApplyMeshBoolean` _target_mesh (struct) _returnvalue_5 (`KismetMathLibrary.MakeTransform` _returnvalue (struct) (`KismetMathLibrary.MakeVector` _returnvalue_6 _returnvalue_6 _returnvalue_6)) _operation (struct) null)
          (`self.ReleaseAllComputeMeshes`))))
    (:`Is Not Valid`
      (bind _returnvalue_7 (`self.AllocateComputeMesh`))
      (bind _returnvalue_8 (`GeometryScriptLibrary_StaticMeshFunctions.CopyMeshFromStaticMesh` _ref_mesh _returnvalue_7 (struct) (struct) null)
        (:`Success`
          (bind _returnvalue_9 (`GeometryScriptLibrary_MeshSimplifyFunctions.ApplySimplifyToTriangleCount` _returnvalue_8 0 (struct) null))
          (bind _returnvalue_10 (`GeometryScriptLibrary_MeshSimplifyFunctions.ApplySimplifyToVertexCount` _returnvalue_9 0 (struct) null))
          (bind _output_get (set `self.Dynamic Mesh Projectile` _returnvalue_10))
          (`GeometryScriptLibrary_MeshBooleanFunctions.ApplyMeshBoolean` _target_mesh (struct) _output_get (`KismetMathLibrary.MakeTransform` _returnvalue (struct) (`KismetMathLibrary.MakeVector` _returnvalue_6 _returnvalue_6 _returnvalue_6)) _operation (make `GeometryScriptMeshBooleanOptions` true) null)
          (`self.ReleaseAllComputeMeshes`))))))

(fn `UserConstructionScript`)